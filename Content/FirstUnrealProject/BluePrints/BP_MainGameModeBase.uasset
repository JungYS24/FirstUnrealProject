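; BP_MainGameModeBase is a game mode Blueprint that serves as a scratchpad of basic Blueprint scripting examples.
; Disconnected, Korean-labeled snippets demonstrate function calls, variables, boolean logic, switch and branch flow, comparison and arithmetic, mostly shown through Print String.
; GetNumberValue is a pass-through example function that returns its input.
; No example is wired to an event and the construction script is empty, so none of this logic runs.
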(fn `GetNumberValue`
  (params (NewValue :type Integer))
  (returns (ResultValue :type Integer))
  (return NewValue))

(fn `UserConstructionScript`)